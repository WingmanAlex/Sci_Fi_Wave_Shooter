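; Tank character Blueprint that equips a Gatling gun as its primary weapon at BeginPlay and adds two cooldown-gated abilities.
; Q spawns a Ground Smash actor at the character's location, with no server routing.
; E taunts enemy AI through a tagged noise event, running on the server via RPC when pressed on a client.
; A deprecated sphere-overlap taunt remains with an empty loop.
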(event Custom|SERVER_Taunt
  ;[0 0.2307 0.4072] Taunt Enemy AI
  (if (Variables|Default|GetIsEReady)
    (Variables|Default|SetIsEReady false)
    (Class|AISenseHearing|ReportNoiseEvent (Transformation|GetWorldLocation (Variables|Default|GetCapsuleComponent)) 1.0 self (Variables|Default|GetTauntRange) "Taunt")
    (Utilities|FlowControl|Delay (Variables|Default|GetAbilityECooldown))
    (Variables|Default|SetIsEReady true)))

(event EventBeginPlay
  (|CallParentFunction)
  (bind _returnvalue (Game|SpawnActorfromClass "/Game/Blueprints/Weapons/BPC_GatlingGun.BPC_GatlingGun_C" (Math|Transform|MakeTransform "0, 0, 0" "0, 0, 0" "1,1,1") "Undefined" 0 0))
  (Variables|Default|SetPrimaryWeapon _returnvalue)
  (Transformation|AttachComponentToComponent (Variables|Default|GetWeapon) (Variables|Character|GetMesh) "WeaponSocket" "SnapToTarget" "SnapToTarget" "SnapToTarget" true))

(event Input|ActionEvents|InputActionAbilityQ
  (params (Key :type Key%20Structure))
  ;[0 0.5572 1] Ability Ground Smash
  (:Pressed
    (if (Variables|Default|GetIsQReady)
      (Game|SpawnActorfromClass "/Game/Blueprints/Ability/BP_GroundSmash.BP_GroundSmash_C" (Math|Transform|MakeTransform (Transformation|GetActorLocation) "0, 0, 0" "1,1,1") "Undefined" 0 0)
      (Variables|Default|SetIsQReady false)
      (Utilities|FlowControl|Delay (Variables|Default|GetAbilityQCooldown))
      (Variables|Default|SetIsQReady true))))

(event Input|ActionEvents|InputActionAbilityE
  (params (Key :type Key%20Structure))
  ;[0 0.2307 0.4072] Taunt Enemy AI
  (:Pressed
    (Networking|SwitchHasAuthority
      (:Authority
        (if (Variables|Default|GetIsEReady)
          (Variables|Default|SetIsEReady false)
          (Class|AISenseHearing|ReportNoiseEvent (Transformation|GetWorldLocation (Variables|Default|GetCapsuleComponent)) 1.0 self (Variables|Default|GetTauntRange) "Taunt")
          (Utilities|FlowControl|Delay (Variables|Default|GetAbilityECooldown))
          (Variables|Default|SetIsEReady true)))
      (:Remote
        (CallFunction|SERVERTaunt)))))

(fn ConstructionScript
  (|CallParentFunction))

(fn DEPRECATEDTAUNTABILITY
  (params (ScanLocation :type Vector) (SphereRadius :type Float%20%28single-precision%29))
  ;[1 1 1] Overlapping Enemies go to this enemy
  (bind _outactors (Collision|SphereOverlapActors ScanLocation SphereRadius (Utilities|Array|MakeArray "ObjectTypeQuery4") "/Game/Spawn_System/Blueprints/Example_AI/BP_Ai_Master.BP_Ai_Master_C"))
  (for _array_element _outactors
    _))
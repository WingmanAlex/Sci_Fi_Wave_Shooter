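; Marine character class that starts with an assault rifle and adds a grenade throw and a work-in-progress Q ability.
; Holding E runs timelines that pitch the launch point and move a tracer to the predicted projectile impact.
; Release launches the grenade along that arc and destroys the tracer.
; Q, labelled as a taunt, sends a fire rate modifier to the primary weapon, gated by a cooldown.
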(event EventBeginPlay
  ;[1 1 1] Begin Play / Attach Start Weapon
  (bind _returnvalue (Game|SpawnActorfromClass "/Game/Blueprints/Weapons/BPC_AssaultRifle.BPC_AssaultRifle_C" (Math|Transform|MakeTransform "0, 0, 0" "0, 0, 0" "1,1,1") "Undefined" 0 0))
  (Variables|Default|SetPrimaryWeapon _returnvalue)
  (Transformation|AttachComponentToComponent (Variables|Default|GetWeapon) (Variables|Character|GetMesh) "WeaponSocket" "SnapToTarget" "SnapToTarget" "SnapToTarget" true))

(event Input|ActionEvents|InputActionAbilityQ
  (params (Key :type Key%20Structure :default "None"))
  ;[0 0.5572 1] Grenade Ability
  ;;[1 1 1] TAUNT ABILITY WIP
  (:Pressed
    (if (Variables|Default|GetAbilityQReady)
      (Class|BPIFireRateModifier|FireRateModifier(Message) (Variables|Default|GetPrimaryWeapon) 0.001)
      (Variables|Default|SetAbilityQReady false)
      (Utilities|FlowControl|Delay (Variables|Default|GetAbilityQCoolDown))
      (Variables|Default|SetAbilityQReady true))))

(event Input|ActionEvents|InputActionAbilityE
  (params (Key :type Key%20Structure :default "None"))
  (bind _granade_launch_point (Variables|Default|GetGranade%20Launch%20Point))
  (bind _returnvalue (Transformation|GetWorldRotation _granade_launch_point))
  ;[0 0.5572 1] Grenade Ability
  ;;[0.5052 0.879 1] Tracer Movement
  (:Pressed
    (Utilities|FlowControl|Sequence
      (:then_0
        (CallFunction|SpawnTracer))
      (:then_1
        ;;[0.4869 0.9502 1] Grenade Arc Movement
        (bind _arcpath (Timeline|GranadeArc PlayFromStart)
          (:Update
            (Transformation|SetWorldRotation _granade_launch_point (Math|Rotator|MakeRotator (.roll _returnvalue) _arcpath (.yaw _returnvalue)) false false))))
      (:then_2
        (Timeline|TracerLocation PlayFromStart
          (:Update
            (CallFunction|TracerMovement))))))
  (:Released
    (Utilities|FlowControl|Sequence
      (:then_0
        (Timeline|GranadeArc Stop))
      (:then_1
        (CallFunction|SpawnGrenade))
      (:then_2
        (Timeline|TracerLocation Stop))
      (:then_3
        (Actor|DestroyActor (Variables|Default|GetTracerReference))))))

(event Input|MouseEvents|LeftMouseButton
  (params (Key :type Key%20Structure :default "None"))
  ;[1 0 0] DEFICATED
)

(fn ConstructionScript
  (|CallParentFunction)
  (Rendering|Material|SetVectorParameterValueonMaterials (Variables|Default|GetSign) "ColorParam" "0.000000,0.100000,1.000000"))

(fn SpawnTracer
  (bind _returnvalue (Game|SpawnActorfromClass "/Game/Blueprints/Weapons/Utilities/BP_GrenadeTracer.BP_GrenadeTracer_C" (Math|Transform|MakeTransform (Transformation|GetWorldLocation (Variables|Default|GetGranade%20Launch%20Point))) "Undefined" 0 0))
  (Variables|Default|SetTracerReference _returnvalue))

(fn TracerMovement
  (bind _granade_launch_point (Variables|Default|GetGranade%20Launch%20Point))
  (bind _outhit (Class|GameplayStatics|BlueprintPredictProjectilePathbyTraceChannel (Transformation|GetWorldLocation _granade_launch_point) (* (Math|Vector|GetForwardVector _granade_launch_point) (Variables|Default|GetThrowStrength)) true 0.0 "ECC_WorldDynamic" false 0 "None"))
  (Transformation|SetWorldLocation (Variables|/Game/Blueprints/Weapons/Utilities/BP_GrenadeTracer.BP_GrenadeTracer_C|GetDefaultSceneRoot (Variables|Default|GetTracerReference)) (.location _outhit) false false))

(fn SpawnGrenade
  (bind _granade_launch_point (Variables|Default|GetGranade%20Launch%20Point))
  (bind _returnvalue (Transformation|GetWorldRotation _granade_launch_point))
  (bind _returnvalue_2 (Game|SpawnActorfromClass "/Game/Blueprints/Ability/BP_GranadeAbility.BP_GranadeAbility_C" (Math|Transform|MakeTransform (Transformation|GetWorldLocation _granade_launch_point) (Math|Rotator|MakeRotator (.roll _returnvalue) 0.0 (.yaw _returnvalue)) "0.200000,0.200000,0.200000") "Undefined" 0 (* (Math|Vector|GetForwardVector _granade_launch_point) (Variables|Default|GetThrowStrength)) 0))
  (Variables|/Game/Blueprints/Ability/BP_GranadeAbility.BP_GranadeAbility_C|SetTracer _returnvalue_2 (Variables|Default|GetTracerReference))
  (Transformation|SetWorldRotation (Variables|Default|GetGranade%20Launch%20Point) (Transformation|GetWorldRotation (Variables|Default|GetCapsuleComponent)) false false))

(fn ShootParticle+Sound
  (Audio|PlaySoundatLocation 0 (Transformation|GetWorldLocation (Variables|Default|GetWeapon)) "0, 0, 0" 2.0 1.0 0.0 0 0 0) ; Play the beautiful shooting sound
)
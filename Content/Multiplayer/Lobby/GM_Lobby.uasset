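; Lobby GameMode for multiplayer that tracks connected players, map settings and character availability before launching the match.
; On post-login it registers each PC_Lobby, pulls server details from GI_GameInfo, and spawns a default character at a random PlayerStart.
; EveryoneUpdate rebroadcasts player and character lists, refreshes the host's kick list, and sets start readiness from character selection.
; It also handles character swaps, kicks, logouts, map-setting changes and servertravel by map ID.
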(event Custom|SwapCharacter
  (params (PlayerController :type Player%20Controller%20Object%20Reference) (CharacterClass :type Character%20Class%20Reference) (ChangedStatus :type Boolean))
  (bind _returnvalue (Pawn|GetControlledPawn PlayerController))
  (bind _spawnpoints (Variables|ServerSettings|GetSpawnPoints))
  ;[1 1 1] Destroys old character, possesses new character from char select screen
  (if (not ChangedStatus)
    (Utilities|IsValid _returnvalue
      (:Is%20Valid
        (Actor|DestroyActor _returnvalue))
      (:Is%20Not%20Valid
        (bind _returnvalue_2 (Game|SpawnActorfromClass CharacterClass (Transformation|GetActorTransform (Utilities|Array|Get(acopy) _spawnpoints (Math|Random|RandomIntegerinRange 0 (- (Utilities|Array|Length _spawnpoints) 1)))) "Undefined" 0 0))
        (Pawn|Possess PlayerController _returnvalue_2)))))

(event Custom|EveryoneUpdate
  (bind _allplayercontrollers (Variables|ServerSettings|GetAllPlayerControllers))
  ;[1 1 1] Updates lobby info for players.
  (bind _output_get (Variables|ServerSettings|SetCurrentPlayers (Utilities|Array|Length (Variables|ServerSettings|GetAllPlayerControllers))))
  (if (> _output_get 0)
    (Utilities|Array|Clear (Variables|ServerSettings|GetConnectedPlayers))
    (for _array_element _allplayercontrollers
      (bind _aspc_lobby (Utilities|Casting|CastToPC_Lobby _array_element))
      (Utilities|Array|Add (Variables|ServerSettings|GetConnectedPlayers) (Variables|/Game/Multiplayer/Lobby/PC_Lobby.PC_Lobby_C|GetPlayerSettings _aspc_lobby))
      (Default|UpdateNumberOfPlayers _aspc_lobby (Variables|ServerSettings|GetCurrentPlayers) (Variables|ServerSettings|GetMaxPlayers)))
    (for _array_element_2 _allplayercontrollers
      (bind _aspc_lobby_2 (Utilities|Casting|CastToPC_Lobby _array_element_2))
      (Default|AddPlayerInfo _aspc_lobby_2 (Variables|ServerSettings|GetConnectedPlayers))
      (Default|UpdateAvailableCharacters _aspc_lobby_2 (Variables|ServerSettings|GetAvailableCharacters))
      (CallFunction|AddtoKickList))
    (bind _array_element_3 (Utilities|Array|ForEachLoopwithBreak (Variables|ServerSettings|GetConnectedPlayers))
      (:LoopBody
        (if (== (.MyPlayerCharacter (Utilities|Struct|BreakS_PlayerInfo _array_element_3)) "/Game/Spawn_System/Blueprints/Character/BP_ThirdPersonCharacter.BP_ThirdPersonCharacter_C")
          (Variables|ServerSettings|SetCanWeStart? false)
          (CallFunction|CannotStartGame)
          (else
            (Variables|ServerSettings|SetCanWeStart? true)))))))

(event Custom|LaunchTheGame
  (bind _returnvalue (Game|GetPlayerController 0))
  ;[1 1 1] Launch game with selected level.
  (Input|SetInputModeGameOnly _returnvalue)
  (switch int (Variables|ServerSettings|GetGM_MapID) ; Add pins for additional maps
    (:0
      (Development|ExecuteConsoleCommand "servertravel AliMap" _returnvalue) ; Without file path
    )
    (:1
      (Development|ExecuteConsoleCommand "servertravel JohanMap" _returnvalue) ; Without file path
    )
    (:2
      (Development|ExecuteConsoleCommand "servertravel AlexMap2" _returnvalue) ; Without file path
    )
    (:3
      (Development|ExecuteConsoleCommand "servertravel AldoMap" _returnvalue) ; Without file path
    )
    (:4
      (Development|ExecuteConsoleCommand "servertravel AldoMap" _returnvalue) ; Without file path
    )))

(event Custom|RespawnPlayer
  (params (PlayerController :type Player%20Controller%20Object%20Reference))
  (bind _returnvalue (Pawn|GetControlledPawn PlayerController))
  (bind _spawnpoints (Variables|ServerSettings|GetSpawnPoints))
  ;[1 1 1] Spawn player as base character when in Lobby / Updates lobby.
  (Utilities|IsValid _returnvalue
    (:Is%20Valid
      (Actor|DestroyActor _returnvalue))
    (:Is%20Not%20Valid
      _))
  (bind _returnvalue_2 (Game|SpawnActorfromClass "/Game/Spawn_System/Blueprints/Character/BP_ThirdPersonCharacter.BP_ThirdPersonCharacter_C" (Transformation|GetActorTransform (Utilities|Array|Get(acopy) _spawnpoints (Math|Random|RandomIntegerinRange 0 (- (Utilities|Array|Length _spawnpoints) 1)))) "Undefined" 0 0))
  (Pawn|Possess PlayerController _returnvalue_2)
  (CallFunction|EveryoneUpdate))

(event Custom|AddToKickList
  ;[1 1 1] Add player to kick list if game settings is open
  (bind _aspc_lobby (Utilities|Casting|CastToPC_Lobby (Game|GetPlayerController 0)))
  (Utilities|IsValid (Variables|/Game/Multiplayer/Lobby/PC_Lobby.PC_Lobby_C|GetLobbyMenuRef _aspc_lobby)
    (:Is%20Valid
      (if (Widget|IsVisible (Variables|/Game/Blueprints/UI/Lobby/WBP_LobbyMenu.WBP_LobbyMenu_C|GetWBP_GameSettings (Variables|/Game/Multiplayer/Lobby/PC_Lobby.PC_Lobby_C|GetLobbyMenuRef _aspc_lobby)))
        (Default|FillPlayersWindow (Variables|/Game/Blueprints/UI/Lobby/WBP_LobbyMenu.WBP_LobbyMenu_C|GetWBP_GameSettings (Variables|/Game/Multiplayer/Lobby/PC_Lobby.PC_Lobby_C|GetLobbyMenuRef _aspc_lobby)))))))

(event Custom|CannotStartGame
  ;[1 1 1] Updates lobby info for players.
  (Utilities|Array|ForEachLoopwithBreak (Variables|ServerSettings|GetConnectedPlayers)) ; enters at Break
)

(event Custom|ServerUpdateGameSettings
  (params (MapImage :type Texture%202D%20Object%20Reference) (MapName :type Text) (MapTime :type Text) (MapID :type Integer))
  ;[1 1 1] Server changes, updates the client's lobby info.
  (Variables|ServerSettings|SetGM_MapImage MapImage)
  (Variables|ServerSettings|SetGM_MapName MapName)
  (Variables|ServerSettings|SetGM_MapTime MapTime)
  (Variables|ServerSettings|SetGM_MapID MapID)
  (for _array_element (Variables|ServerSettings|GetAllPlayerControllers)
    (bind _aspc_lobby (Utilities|Casting|CastToPC_Lobby _array_element))
    (Default|UpdateLobbySettings _aspc_lobby (Variables|ServerSettings|GetGM_MapImage) (Variables|ServerSettings|GetGM_MapName) (Variables|ServerSettings|GetGM_MapTime))))

(event Custom|YouHaveBeenKicked
  (params (PlayerID :type Integer))
  ;[1 1 1] Kick selected player from lobby.
  (Default|Kicked (.AsPC%20Lobby (Utilities|Casting|CastToPC_Lobby (Utilities|Array|Get(acopy) (Variables|ServerSettings|GetAllPlayerControllers) PlayerID)))))

(event EventPostLogin
  (params (NewPlayer :type Player%20Controller%20Object%20Reference))
  ;[1 1 1] Event OnPostLogin - Construct players, copy from PC to GM.
  (Networking|SwitchHasAuthority ; Runs script bsed on whether it's linked to client or host.
    (:Authority
      (Utilities|Array|Add (Variables|ServerSettings|GetAllPlayerControllers) NewPlayer)
      (bind _outactors (Actor|GetAllActorsOfClass "/Script/Engine.PlayerStart")) ; Assign specific spawn points based on tags, if used for teams.
      (Variables|ServerSettings|SetSpawnPoints _outactors)
      (bind _asgi_game_info (Utilities|Casting|CastToGI_GameInfo (Game|GetGameInstance)))
      (Variables|ServerSettings|SetServerName (Variables|/Game/Multiplayer/GI_GameInfo.GI_GameInfo_C|GetServerName _asgi_game_info))
      (Variables|ServerSettings|SetMaxPlayers (Variables|/Game/Multiplayer/GI_GameInfo.GI_GameInfo_C|GetMaxPlayers _asgi_game_info))
      (bind _aspc_lobby (Utilities|Casting|CastToPC_Lobby NewPlayer))
      (Default|InitialSetup _aspc_lobby)
      (Default|SetupLobbyMenu _aspc_lobby (Variables|ServerSettings|GetServerName))
      (Default|UpdateLobbySettings _aspc_lobby (Variables|ServerSettings|GetGM_MapImage) (Variables|ServerSettings|GetGM_MapName) (Variables|ServerSettings|GetGM_MapTime)) ; Set GM version of the PC_Lobby variables
      (CallFunction|RespawnPlayer NewPlayer))))

(event EventOnLogout
  (params (ExitingController :type Controller%20Object%20Reference))
  (bind _allplayercontrollers (Variables|ServerSettings|GetAllPlayerControllers))
  ;[1 1 1] Event Logout, removes PC, and connected player info. Updates available character.
  (bind (_array_element _array_index) (Utilities|Array|ForEachLoopwithBreak _allplayercontrollers :!label _label)
    (:LoopBody
      (if (== _array_element ExitingController)
        (goto _label Break)))
    (:Completed
      (bind _aspc_lobby (Utilities|Casting|CastToPC_Lobby (Utilities|Array|Get(acopy) _allplayercontrollers _array_index)))
      (Utilities|Array|SetArrayElem (Variables|ServerSettings|GetAvailableCharacters) (Variables|/Game/Multiplayer/Lobby/PC_Lobby.PC_Lobby_C|GetSelectedCharacter _aspc_lobby) false)
      (Utilities|Array|RemoveIndex (Variables|ServerSettings|GetAllPlayerControllers) _array_index)
      (Utilities|Array|RemoveIndex (Variables|ServerSettings|GetConnectedPlayers) _array_index)
      (CallFunction|EveryoneUpdate))))

(fn ConstructionScript)
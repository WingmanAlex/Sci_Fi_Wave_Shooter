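; Multiplayer player controller that hands saved player settings to the game mode and runs the in-game text chat.
; On local BeginPlay it loads the save slot, then passes the settings on for GM_Gameplay to respawn the chosen character, and creates a hidden chat widget.
; Outgoing messages loop through the game mode's controller list, updating each one's chat window with sender name and text.
; The T key toggles chat and cursor visibility.
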(event Custom|PassCharacterInfoToServer
  (params (PlayerSettings :type S%20Player%20Info%20Structure))
  ;[1 1 1] Passes character info / Respaws with selected character / setup chat
  (Variables|Default|SetPlayerSettings PlayerSettings)
  (bind _asgm_gameplay (Utilities|Casting|CastToGM_Gameplay (Game|GetGameMode)))
  (Default|RespawnPlayer _asgm_gameplay self (Utilities|Struct|BreakS_Player_Info (Variables|Default|GetPlayerSettings)))
  (CallFunction|SetupChatWindows))

(event Custom|SetupChatWindows
  ;[1 1 1] Create gameplay chat, add to viewport
  (bind _returnvalue (UserInterface|CreateWidget "/Game/Blueprints/UI/Chat/WBP_GameChat.WBP_GameChat_C"))
  (bind _output_get (Variables|Default|SetGameChatRef _returnvalue))
  (UserInterface|Viewport|AddtoViewport _output_get 0)
  (Widget|SetVisibility (Variables|Default|GetGameChatRef) "Hidden"))

(event Custom|GetChatMessage
  (params (TextToSend :type Text))
  ;[1 1 1] Setup Chat windows / Updates chat in PC.
  (Variables|Default|SetSenderText TextToSend)
  (Variables|Default|SetSenderName (.MyPlayerName (Utilities|Struct|BreakS_Player_Info (Variables|Default|GetPlayerSettings))))
  (bind _asgm_gameplay (Utilities|Casting|CastToGM_Gameplay (Game|GetGameMode)))
  (for _array_element (Variables|/Game/Multiplayer/GM_Gameplay.GM_Gameplay_C|GetAllPlayerControllers _asgm_gameplay)
    (bind _aspc_player_controller (Utilities|Casting|CastToPC_PlayerController _array_element))
    (CallFunction|UpdateChat _aspc_player_controller (Variables|Default|GetSenderName) (Variables|Default|GetSenderText))))

(event Custom|UpdateChat
  (params (SenderName :type Text) (SenderText :type Text))
  ;[1 1 1] UpdateChat window
  (Default|UpdateChatWindow (Variables|/Game/Blueprints/UI/Chat/WBP_GameChat.WBP_GameChat_C|GetWBP_ChatWindow (Variables|Default|GetGameChatRef)) SenderName SenderText))

(event EventBeginPlay
  ;[1 1 1] Loading player info and pass to server side controller
  (if (Pawn|IsLocalController)
    (Viewport|RemoveAllWidgets)
    (CallFunction|LoadGame)
    (CallFunction|PassCharacterInfotoServer (Variables|Default|GetPlayerSettings))))

(event Input|KeyboardEvents|T
  (params (Key :type Key%20Structure))
  (bind _gamechatref (Variables|Default|GetGameChatRef))
  ;[1 1 1] T for Type
  (:Pressed
    (Utilities|FlowControl|FlipFlop
      (:A
        (Variables|Default|SetbShowMouseCursor true)
        (Widget|SetVisibility _gamechatref "Visible"))
      (:B
        (Variables|Default|SetbShowMouseCursor false)
        (Widget|SetVisibility _gamechatref "Collapsed")))))

(fn ConstructionScript)

(fn LoadGame
  (bind _returnvalue (SaveGame|LoadGamefromSlot (Variables|Default|GetPlayerSettingsSave)))
  (bind _assg_player_save_game (Utilities|Casting|CastToSG_PlayerSaveGame _returnvalue))
  (Variables|Default|SetPlayerSettings (Variables|/Game/Multiplayer/SG_PlayerSaveGame.SG_PlayerSaveGame_C|GetS_Player_Info _assg_player_save_game)))
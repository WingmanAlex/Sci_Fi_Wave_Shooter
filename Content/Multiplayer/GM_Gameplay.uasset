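; Multiplayer gameplay GameMode that runs enemy waves, a final extraction countdown and the win screen.
; A looping timer spawns random enemies at random TargetPoints, and clearing the tracked enemy array triggers an intermission before the next, larger wave.
; Once CurrentWave reaches MaxWave, the next start runs only the countdown.
; It also respawns chosen characters at random PlayerStarts, tracks swapped controllers and calls session destruction on logout.
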(event Custom|RespawnPlayer
  (params (PlayerController :type Player%20Controller%20Object%20Reference) (PlayerCharacter :type Character%20Class%20Reference))
  ;[1 1 1] Spawn player with selected character from GP PC.
  (bind _outactors (Actor|GetAllActorsOfClass "/Script/Engine.PlayerStart"))
  (Variables|GameInfo|SetSpawnPoints _outactors)
  (bind _returnvalue (Game|SpawnActorfromClass PlayerCharacter (Transformation|GetActorTransform (Utilities|Array|Get(acopy) (Variables|GameInfo|GetSpawnPoints) (Math|Random|RandomIntegerinRange 0 (- (Utilities|Array|Length (Variables|GameInfo|GetSpawnPoints)) 1)))) "Undefined" 0 0))
  (Pawn|Possess PlayerController _returnvalue))

(event Custom|SpawnWave
  ;[1 0 0.8805] Waves and Spawning
  ;;[1 1 1] SpawnWave event
  (CallFunction|SpawnEnemy))

(event Custom|EndWave
  ;[1 0 0.8805] Waves and Spawning
  ;;[1 1 1] EndWave event
  (Development|PrintString "Wave end!" true true "(R=0.856883,G=1.000000,B=0.000000,A=1.000000)" (Variables|WaveSettings|GetIntermissionTime))
  (CallFunction|Intermission))

(event Custom|Intermission
  ;[1 0 0.8805] Waves and Spawning
  ;;[1 1 1] Intermission event
  (Utilities|FlowControl|Delay (Variables|WaveSettings|GetIntermissionTime))
  (CallFunction|StartNewWave))

(event Custom|FinalWaveCount
  ;[1 0 0.8805] Waves and Spawning
  ;;[1 1 1] Final Wave
  (bind _returnvalue (Utilities|Time|SetTimerbyFunctionName 0 "Countdown" 1.0 true)))

(event Custom|EndGame
  ;[1 0 0.8805] Waves and Spawning
  ;;[1 1 1] EndGame
  (Utilities|Time|ClearandInvalidateTimerbyHandle (stale Custom|FinalWaveCount _returnvalue))
  (Default|CallStopMovement)
  (bind _returnvalue (UserInterface|CreateWidget "/Game/Blueprints/UI/Player/WBP_WinScreen.WBP_WinScreen_C"))
  (UserInterface|Viewport|AddtoViewport _returnvalue 0))

(event EventBeginPlay
  ;[1 0.7384 0] Event BeginPlay
  (bind _returnvalue (UserInterface|CreateWidget "/Game/Blueprints/UI/Player/WBP_WaveInfo.WBP_WaveInfo_C" 0 (Variables|WaveSettings|GetCurrentWave)))
  (bind _output_get (Variables|Default|SetWaveInfoRef _returnvalue))
  (UserInterface|Viewport|AddtoViewport _returnvalue 0)
  ;[1 0 0.8805] Waves and Spawning
  ;;[1 1 1] Start Wave
  (Utilities|FlowControl|Delay 1.0)
  (CallFunction|StartNewWave))

(event EventOnSwapPlayerControllers
  (params (OldPC :type Player%20Controller%20Object%20Reference) (NewPC :type Player%20Controller%20Object%20Reference))
  ;[1 1 1] Tracks connected player controllers
  (Utilities|Array|Add (Variables|GameInfo|GetAllPlayerControllers) NewPC))

(event EventOnLogout
  (params (ExitingController :type Controller%20Object%20Reference))
  ;[1 1 1] Event On logout - Destroy session caller in GI instance.
  (bind _aspc_player_controller (Utilities|Casting|CastToPC_PlayerController ExitingController))
  (Default|DestroySessionCaller (.AsGI%20Game%20Info (Utilities|Casting|CastToGI_GameInfo (Game|GetGameInstance))) _aspc_player_controller))

(fn ConstructionScript)

(fn StartNewWave
  (Development|PrintString "Starting wave!" true true "(R=1.000000,G=0.000000,B=0.059079,A=1.000000)")
  (if (< (Variables|WaveSettings|GetCurrentWave) (Variables|WaveSettings|GetMaxWave))
    ;[1 1 1] SpawnWave
    (Math|Integer|IncrementInt (Variables|WaveSettings|GetCurrentWave)
      (:%20%20
        (Default|CallSendWave)
        (CallFunction|IncreaseWaveDifficulty)
        (Utilities|Time|SetTimerbyFunctionName 0 "SpawnWave" (Variables|WaveSettings|GetSpawnFrequency) true 1.0)))
    (else
      ;[1 1 1] Final Wave event
      (if (== (Variables|WaveSettings|GetCurrentWave) (Variables|WaveSettings|GetMaxWave))
        (Default|CallSendWave)
        (CallFunction|FinalWaveCount)))))

(fn SpawnEnemy
  (bind _spawnpoint (CallFunction|GetRandomSpawnPoint))
  (Utilities|IsValid _spawnpoint
    (:Is%20Valid
      (bind _returnvalue (Game|SpawnActorfromClass (Utilities|Array|Get(acopy) (Variables|WaveSettings|GetEnemyClasses) (Math|Random|RandomIntegerinRange 0 (Utilities|Array|LastIndex (Variables|WaveSettings|GetEnemyClasses)))) (Transformation|GetActorTransform _spawnpoint) "AdjustIfPossibleButAlwaysSpawn" 0 0)) ; Spawn Enemy...
      (Utilities|IsValid _returnvalue
        (:Is%20Valid
          (Utilities|Array|Add (Variables|WaveSettings|GetEnemyArray) _returnvalue) ; Add spawned enemy to EnemyArray.
          (bind _output_get (Variables|WaveSettings|SetRemainingSpawns (- (Variables|WaveSettings|GetRemainingSpawns) 1)))
          (if (== _output_get 0)
            (Utilities|Time|ClearTimerbyFunctionName 0 "SpawnWave")))))))

(fn GetRandomSpawnPoint
  (bind _outactors (Actor|GetAllActorsOfClass "/Script/Engine.TargetPoint"))
  (return (Utilities|Array|Get(acopy) _outactors (Math|Random|RandomIntegerinRange 0 (Utilities|Array|LastIndex _outactors)))))

(fn RemoveEnemyfromArray
  (params (EnemyToRemove :type BP%20Enemy%20Master%20Object%20Reference%20%28by%20ref%29))
  (Utilities|Array|RemoveItem (Variables|WaveSettings|GetEnemyArray) EnemyToRemove)
  (if (CallFunction|IsWaveComplete)
    (CallFunction|EndWave)))

(fn IsWaveComplete
  (return (and (<= (Utilities|Array|Length (Variables|WaveSettings|GetEnemyArray)) 0) (<= (Variables|WaveSettings|GetRemainingSpawns) 0))))

(fn IncreaseWaveDifficulty
  (bind _output_get (Variables|WaveSettings|SetWaveDifficulty (Math|Float|Round (* (Variables|WaveSettings|GetWaveDifficulty) (Variables|WaveSettings|GetDifficultyMultiplier)))))
  (Variables|WaveSettings|SetRemainingSpawns _output_get))

(fn OnRepCurrentWave)

(fn Countdown
  (Variables|Default|SetExtractionTimer (- (Variables|Default|GetExtractionTimer) 1))
  (Development|PrintString (Utilities|String|ToString(Integer) (Variables|Default|GetExtractionTimer)))
  (if (<= (Variables|Default|GetExtractionTimer) 0)
    (CallFunction|EndGame)))

(fn GetGameplay
  (return 0))
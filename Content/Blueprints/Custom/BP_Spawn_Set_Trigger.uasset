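; BP_Spawn_Set_Trigger is a one-shot trigger that spawns a set of actors when the player character overlaps it.
; The overlap prints a debug string and calls CreateNewSpawns, which passes a DoOnce and loops SpawnVectorArray, spawning at each offset from the trigger's location.
; DestroyOverlap destroys the trigger from inside that loop.
; The live spawn node shows no class; disconnected deprecated code spawns BP_EnemyMaster at a random array entry.
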(event OnComponentBeginOverlap(Trigger)
  (params (OverlappedComponent :type Primitive%20Component%20Object%20Reference) (OtherActor :type Actor%20Object%20Reference) (OtherComp :type Primitive%20Component%20Object%20Reference) (OtherBodyIndex :type Integer) (bFromSweep :type Boolean) (SweepResult :type Hit%20Result%20Structure%20%28by%20ref%29))
  ;[0.07721 0 1] Overlap code
  (if (== OtherActor (Game|GetPlayerCharacter 0))
    (Development|PrintString "Overlapping" true true "(R=0.000000,G=1.000000,B=0.052976,A=1.000000)")
    (CallFunction|CreateNewSpawns)))

(event Custom|CreateNewSpawns
  ;[1 0 0.9168] Spawn at transform
  (Utilities|FlowControl|DoOnce false
    (:Completed
      (for _array_element (Variables|Default|GetSpawnVectorArray)
        (Game|SpawnActorfromClass "/Script/Engine.TargetPoint" (Math|Transform|MakeTransform (+ (.Location (Math|Transform|BreakTransform (Transformation|GetActorTransform))) (.Location (Math|Transform|BreakTransform _array_element))) "0, 0, 0" "1,1,1") "AdjustIfPossibleButAlwaysSpawn" 0 0)
        (CallFunction|DestroyOverlap)))))

(event Custom|DestroyOverlap
  ;[0 0.9776 1] Destroy Overlapper
  (Actor|DestroyActor))

(fn ConstructionScript)
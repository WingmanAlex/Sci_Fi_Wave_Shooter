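; Trigger actor that scatters spawn markers around itself when the player walks into it.
; An overlap with player character 0 prints a debug message and calls CreateNewSpawns, gated by a DoOnce.
; That event spawns four TargetPoint actors at random navigable locations within a fixed radius of the trigger, keeping its rotation, then destroys the trigger.
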(event OnComponentBeginOverlap(Trigger)
  (params (OverlappedComponent :type Primitive%20Component%20Object%20Reference) (OtherActor :type Actor%20Object%20Reference) (OtherComp :type Primitive%20Component%20Object%20Reference) (OtherBodyIndex :type Integer) (bFromSweep :type Boolean) (SweepResult :type Hit%20Result%20Structure%20%28by%20ref%29))
  (if (== OtherActor (Game|GetPlayerCharacter 0))
    (Development|PrintString "Overlapping" true true "(R=0.000000,G=1.000000,B=0.052976,A=1.000000)")
    (CallFunction|CreateNewSpawns)))

(event Custom|CreateNewSpawns
  (bind _returnvalue (Transformation|GetActorTransform))
  (bind _returnvalue_2 (Transformation|GetActorTransform))
  (bind _returnvalue_3 (Transformation|GetActorTransform))
  (bind _returnvalue_4 (Transformation|GetActorTransform))
  (Utilities|FlowControl|DoOnce false
    (:Completed
      (Game|SpawnActorfromClass "/Script/Engine.TargetPoint" (Math|Transform|MakeTransform (.RandomLocation (Class|NavigationSystemV1|GetRandomPointinNavigableRadius (.location _returnvalue_2) 2e+03 0 0)) (.rotation _returnvalue_2) "1,1,1") "AdjustIfPossibleButAlwaysSpawn" 0 0)
      (Game|SpawnActorfromClass "/Script/Engine.TargetPoint" (Math|Transform|MakeTransform (.RandomLocation (Class|NavigationSystemV1|GetRandomPointinNavigableRadius (.location _returnvalue_4) 2e+03 0 0)) (.rotation _returnvalue_4) "1,1,1") "AdjustIfPossibleButAlwaysSpawn" 0 0)
      (Game|SpawnActorfromClass "/Script/Engine.TargetPoint" (Math|Transform|MakeTransform (.RandomLocation (Class|NavigationSystemV1|GetRandomPointinNavigableRadius (.location _returnvalue) 2e+03 0 0)) (.rotation _returnvalue) "1,1,1") "AdjustIfPossibleButAlwaysSpawn" 0 0)
      (Game|SpawnActorfromClass "/Script/Engine.TargetPoint" (Math|Transform|MakeTransform (.RandomLocation (Class|NavigationSystemV1|GetRandomPointinNavigableRadius (.location _returnvalue_3) 2e+03 0 0)) (.rotation _returnvalue_3) "1,1,1") "AdjustIfPossibleButAlwaysSpawn" 0 0)
      (Actor|DestroyActor))))

(fn ConstructionScript)
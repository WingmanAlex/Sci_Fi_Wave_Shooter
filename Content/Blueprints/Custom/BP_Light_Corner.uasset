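; BP_Light_Corner is an interactable light actor that players toggle on and off over the network.
; Interact flips the replicated LightOn flag, with remote instances calling a server RPC and also toggling locally.
; OnRep_LightOn switches the point light's visibility and the bulb's material between wall and emissive, printing the state.
; The flag reads inverted: a true LightOn turns the light off.
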(event Custom|SetLight
  (Networking|SwitchHasAuthority
    (:Authority
      _)
    (:Remote
      (CallFunction|SERVERSetLight)))
  (if (Variables|Default|GetLightOn?)
    (Variables|Default|SetLightOn? false)
    (else
      (Variables|Default|SetLightOn? true))))

(event Custom|SERVER_SetLight
  (if (Variables|Default|GetLightOn?)
    (Variables|Default|SetLightOn? false)
    (else
      (Variables|Default|SetLightOn? true))))

(event EventBeginPlay)

(event Collision|EventActorBeginOverlap
  (params (OtherActor :type Actor%20Object%20Reference)))

(event EventInteract
  (CallFunction|SetLight))

(fn ConstructionScript)

(fn OnRepLightOn?
  (if (Variables|Default|GetLightOn?)
    ;[1 1 1] Lights off
    (Rendering|SetVisibility (Variables|Default|GetPointLight) false false)
    (Rendering|Material|SetMaterial (Variables|Default|GetBulb) 0 "/Game/Spawn_System/Materials/MI_Walls_1.MI_Walls_1")
    (Development|PrintString "Lights Off" true true "(R=1.000000,G=0.157706,B=0.000000,A=1.000000)")
    (else
      ;[1 1 1] Lights on
      (Rendering|SetVisibility (Variables|Default|GetPointLight) true false)
      (Rendering|Material|SetMaterial (Variables|Default|GetBulb) 0 "/Game/Spawn_System/Maps/DemoRoom/Materials/M_Emissive_2.M_Emissive_2")
      (Development|PrintString "Lights On" true true "(R=1.000000,G=0.783689,B=0.000000,A=1.000000)"))))
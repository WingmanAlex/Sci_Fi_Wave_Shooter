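; BP_EnemyChild_Spider is a spider enemy child Blueprint that specializes a parent enemy class.
; Its construction script attaches two collision cylinders to the head and abdomen bones of the mesh, then runs the parent construction script.
; BeginPlay and the SendAttack event only print debug strings, so the spider has no attack logic of its own here.
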(event EventBeginPlay
  (Development|PrintString "I AM ZPIDER"))

(event EventSendAttack
  (Development|PrintString "AttackSetOnChild"))

(fn ConstructionScript
  (Transformation|AttachComponentToComponent (Variables|Default|GetCollisionCylinder2) (Variables|Character|GetMesh) "b_SPR_Head" "KeepRelative" "KeepRelative" "KeepRelative" true)
  (Transformation|AttachComponentToComponent (Variables|Default|GetCollisionCylinder1) (Variables|Character|GetMesh) "b_SPR_Abdomen" "KeepRelative" "KeepRelative" "KeepRelative" true)
  (|CallParentFunction))
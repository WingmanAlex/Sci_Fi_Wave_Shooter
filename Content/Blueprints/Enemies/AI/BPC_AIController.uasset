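; AI controller for enemies that runs the BT_AI behavior tree and picks a player target by threat.
; On the authority, perception updates for player character 0 feed parallel player and threat arrays.
; Sight and damage add stimulus strength unless taunted; hearing acts as a taunt, lifting threat above the current highest.
; These stimuli set the isEnemyAlerted blackboard key, and the highest-threat player becomes PlayerCharacter.
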(event OnTargetPerceptionUpdated(AIPerception)
  (params (Actor :type Actor%20Object%20Reference) (Stimulus :type AI%20Stimulus%20Structure))
  (Networking|SwitchHasAuthority
    (:Authority
      (if (== (Game|GetPlayerCharacter 0) Actor)
        (Variables|Replication|SetAIStimulus Stimulus)
        (if (Utilities|Array|ContainsItem (Variables|Default|GetPlayerSenseArray) Actor)
          _
          (else
            ;[1 1 0.2] Adds player to array
            (Utilities|Array|Add (Variables|Default|GetPlayerSenseArray) Actor)
            (Utilities|Array|Add (Variables|Default|GetThreatArray) 0.0)))
        ;[0 1 1] On sight / Taunt / Damage
        (bind _returnvalue (Class|AIPerceptionSystem|GetSenseClassforStimulus (Variables|Replication|GetAIStimulus)))
        (switch string (Utilities|GetClassDisplayName _returnvalue)
          (:AISense_Hearing
            (bind _output_get (Variables|Default|SetisTaunted (.bsuccessfullysensed (Variables|Replication|GetAIStimulus))))
            (if _output_get
              (Utilities|Array|SetArrayElem (Variables|Default|GetThreatArray) (Variables|Default|GetPlayerIndex) (+ (Variables|Default|GetHighestThreat) 5e+01))
              (AI|Components|Blackboard|SetValueasBool (AI|GetBlackboard 0) (Utilities|Name|MakeLiteralName "isEnemyAlerted") true)
              (CallFunction|GetHighestThreat)
              (else
                (CallFunction|GetHighestThreat))))
          (:AISense_Damage
            (if (not (Variables|Default|GetisTaunted)) :!label _label
              (CallFunction|SetThreat)
              (CallFunction|GetHighestThreat)
              (AI|Components|Blackboard|SetValueasBool (AI|GetBlackboard 0) (Utilities|Name|MakeLiteralName "isEnemyAlerted") (.bsuccessfullysensed (Variables|Replication|GetAIStimulus)))))
          (:AISense_Sight
            (goto _label)))))))

(event Custom|GetHighestThreat
  (bind _playersensearray (Variables|Default|GetPlayerSenseArray))
  (bind _threatarray (Variables|Default|GetThreatArray))
  (bind (_indexofmaxvalue _maxvalue) (Math|Float|MaxOfFloatArray _threatarray))
  (bind _output (Utilities|Array|Get(acopy) _playersensearray _indexofmaxvalue))
  ;[1 1 0.2] Set highest threat player as target
  (Variables|Default|SetHighestThreat _maxvalue)
  (if (not (== (Variables|Default|GetPlayerCharacter) _output))
    (bind _output_get (Variables|Default|SetPlayerCharacter _output))
    (Development|PrintString (Utilities|String|Append "Switched threat: " (Utilities|GetDisplayName _output_get)))))

(event EventBeginPlay
  (AI|RunBehaviorTree "/Game/Blueprints/Enemies/AI/BT_AI.BT_AI"))

(fn ConstructionScript)

(fn SetThreat
  (bind _playerindex (Variables|Default|GetPlayerIndex))
  (bind _threatarray (Variables|Default|GetThreatArray))
  (Utilities|Array|SetArrayElem _threatarray _playerindex (+ (Utilities|Array|Get(acopy) _threatarray _playerindex) (.strength (Variables|Replication|GetAIStimulus)))))
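; Base enemy Blueprint that handles health, melee attacks, stuns and death.
; RepNotify variables drive the logic: each attack-flag change briefly halts movement and schedules a delayed range check that damages the first player.
; When damage empties health, it sends that player random XP and sets the dead flag, which stops AI logic, removes the enemy from GM_Gameplay's array and sets a short lifespan.
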(event EventBeginPlay
  (Variables|Health|SetCurrentHealth (Variables|Health|GetMaxHealth)))

(event EventStunned
  (params (StunTime :type Float%20%28single-precision%29))
  ;[1 1 1] Stun
  (Pawn|Components|CharacterMovement|DisableMovement (Variables|Character|GetCharacterMovement))
  (Utilities|FlowControl|Delay StunTime)
  (Pawn|Components|CharacterMovement|SetMovementMode (Variables|Character|GetCharacterMovement) "MOVE_Walking" 0))

(event Game|Damage|EventAnyDamage
  (params (Damage :type Float%20%28single-precision%29) (DamageType :type Damage%20Type%20Object%20Reference) (InstigatedBy :type Controller%20Object%20Reference) (DamageCauser :type Actor%20Object%20Reference))
  ;[1 1 1] Damage Event (Checks if dead onRep)
  (Variables|Health|SetCurrentHealth (- (Variables|Health|GetCurrentHealth) Damage)))

(event EventSetAttack
  (params (isAttack :type Boolean))
  ;[1 1 1] Attack when in range
  (if isAttack
    (Variables|States|SetisAttack true)
    (else
      (Utilities|FlowControl|Delay (Variables|Default|GetAttackAnimTime))
      (Variables|States|SetisAttack false))))

(fn ConstructionScript)

(fn OnRepIsDead
  (States|SetEnemyDeath))

(fn OnRepCurrentHealth
  (if (<= (Variables|Health|GetCurrentHealth) 0.0)
    (CallFunction|SetSendXP)
    (Variables|States|SetIsDead true)))

(fn SetEnemyDeath
  (Variables|/Script/Engine.CharacterMovementComponent|SetbUseControllerDesiredRotation (Variables|Character|GetCharacterMovement) false)
  (AI|Logic|StopLogic (Variables|/Script/AIModule.AIController|GetBrainComponent (AI|GetAIController 0)) "")
  (bind _asgm_gameplay (Utilities|Casting|CastToGM_Gameplay (Game|GetGameMode)))
  (Default|RemoveEnemyfromArray _asgm_gameplay self)
  (Actor|SetLifeSpan 5.0))

(fn SetSendXP
  (Class|BPIExperience|SetRecieveXP(Message) (Game|GetPlayerCharacter 0) (Math|Conversions|ToFloat(Integer) (Math|Random|RandomIntegerinRange (Variables|Reward|GetMinXP_Reward) (Variables|Reward|GetMaxXP_Reward)))))

(fn OnRepIsAttack
  (Utilities|Time|SetTimerbyFunctionName 0 "DoDamage" 0.8)
  (Pawn|Components|CharacterMovement|DisableMovement (Variables|Character|GetCharacterMovement))
  (Utilities|Time|SetTimerbyFunctionName 0 "SetMovementMode" 0.5))

(fn DoDamage
  (bind _returnvalue (Game|GetPlayerCharacter 0))
  (if (<= (Math|Vector|VectorLength (- (Transformation|GetActorLocation) (Transformation|GetActorLocation _returnvalue))) (Variables|Default|GetMeleeRange))
    (Game|Damage|ApplyDamage _returnvalue (Variables|Default|GetBaseDamage) 0 self)))

(fn SetMovementMode
  (Pawn|Components|CharacterMovement|SetMovementMode (Variables|Character|GetCharacterMovement) "MOVE_Walking" 0))
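; Assault rifle weapon Blueprint that handles automatic firing.
; BeginPlay takes FireRate from WeaponStruct as the timer interval.
; SetFire calls TESTBullet on both start and stop, then starts or clears its looping timer; a FireBullet timer is left unconnected.
; The unfinished FireRateModifier overrides FireRate without restarting the timer or restoring the old value, and SwitchFireRate is empty.
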(event EventSetFire
  (params (IsFiring :type Boolean))
  ;[1 1 1] Shooting Behaviour
  (CallFunction|TESTBullet)
  (if IsFiring
    (bind _returnvalue (Utilities|Time|SetTimerbyFunctionName 0 "TESTBullet" (Variables|Default|GetFireRate) true))
    (Variables|Default|SetGunTimer _returnvalue)
    (else
      (Utilities|Time|ClearandInvalidateTimerbyHandle (Variables|Default|GetGunTimer)))))

(event EventFireRateModifier
  (params (FireRateBoost :type Float%20%28single-precision%29))
  ;[1 0 0] NOTDONE
  (Variables|Default|SetFireRateBoostActive true)
  (bind _output_get (Variables|Default|SetFireRate FireRateBoost))
  (Development|PrintString (Utilities|String|ToString(Float) _output_get)))

(event EventBeginPlay
  ;[1 1 1] Set local variables
  (bind _output_get (Variables|Default|SetWeaponStruct (Variables|Default|GetWeaponStruct)))
  (Variables|Default|SetFireRate (.firerate _output_get)))

(fn ConstructionScript
  (|CallParentFunction))

(fn SwitchFireRate)
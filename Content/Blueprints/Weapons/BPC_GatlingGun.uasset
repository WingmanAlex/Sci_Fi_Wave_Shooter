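; Gatling gun weapon component that adds spin-up and overheating to its parent's firing and reload logic.
; A timeline scaled by ChargeTime drives the charge and, at full charge, starts a FireRate timer that calls FireBullet, adding heat per shot.
; Releasing the trigger reverses the charge and cools heat through a per-frame Delay loop.
; Overheating blocks firing and reloading until heat drains to zero at a fixed step.
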(event Custom|DecreaseHeat
  ;[1 1 1] Decrease Heat
  (if (> (Variables|Default|GetCurrentHeat) 0.0) :!label _label
    (if (Variables|Default|GetIsOverheated)
      (bind _output_get (Variables|Default|SetCurrentHeat (Math|Float|Clamp(Float) (- (Variables|Default|GetCurrentHeat) 0.01)) :!label _label_2))
      (Utilities|FlowControl|Delay (Utilities|Time|GetWorldDeltaSeconds))
      (if (<= _output_get 0.0) ; keep reducing hit each world delta second until no longer overheated
        (Variables|Default|SetIsOverheated false)
        (else
          (goto _label_2)))
      (else
        ;;[1 1 1] decreasing heat when not overheated
        (Variables|Default|SetCurrentHeat (Math|Float|Clamp(Float) (- (Variables|Default|GetCurrentHeat) (* (Variables|Default|GetFireRate) 0.1))))
        (Utilities|FlowControl|Delay (Utilities|Time|GetWorldDeltaSeconds))
        (if (and (not (Variables|Default|GetIsFiringBullets)) (not (Variables|Default|GetIsOverheated))) ; keep reducing heat each delta second until you start shooting or you are overheated
          (Development|PrintString "Decreasing Heat")
          (goto _label))))))

(event EventSetFire
  (params (IsShooting :type Boolean))
  ;[1 1 1] Shoot/Stop Shoot
  (if (Variables|Default|GetIsReloading) ; Decrease Heat when reloading
    ;[1 1 1] Decrease Heat
    (if (> (Variables|Default|GetCurrentHeat) 0.0) :!label _label
      (if (Variables|Default|GetIsOverheated)
        (bind _output_get (Variables|Default|SetCurrentHeat (Math|Float|Clamp(Float) (- (Variables|Default|GetCurrentHeat) 0.01)) :!label _label_2))
        (Utilities|FlowControl|Delay (Utilities|Time|GetWorldDeltaSeconds))
        (if (<= _output_get 0.0) ; keep reducing hit each world delta second until no longer overheated
          (Variables|Default|SetIsOverheated false)
          (else
            (goto _label_2)))
        (else
          ;;[1 1 1] decreasing heat when not overheated
          (Variables|Default|SetCurrentHeat (Math|Float|Clamp(Float) (- (Variables|Default|GetCurrentHeat) (* (Variables|Default|GetFireRate) 0.1))))
          (Utilities|FlowControl|Delay (Utilities|Time|GetWorldDeltaSeconds))
          (if (and (not (Variables|Default|GetIsFiringBullets)) (not (Variables|Default|GetIsOverheated))) ; keep reducing heat each delta second until you start shooting or you are overheated
            (Development|PrintString "Decreasing Heat")
            (goto _label)))))
    (elif IsShooting
      (if (not (Variables|Default|GetIsOverheated))
        (Components|Timeline|SetPlayRate (Variables|Default|GetChargeUpGun) (/ 2.0 (Variables|Default|GetChargeTime)))
        (bind _alpha (Timeline|ChargeUpGun Play)
          (:Update
            (bind _output_get_2 (Variables|Default|SetCurrentCharge (Math|Float|Lerp 0.0 1.0 _alpha)))
            (if (>= _output_get_2 1.0)
              (bind _returnvalue (Utilities|Time|SetTimerbyFunctionName 0 "FireBullet" (Variables|Default|GetFireRate) (not (Variables|Default|GetIsReloading))))
              (Variables|Default|SetGunTimer _returnvalue)))))
      (else
        (Utilities|Time|ClearandInvalidateTimerbyHandle (Variables|Default|GetGunTimer))
        (Utilities|FlowControl|Sequence
          (:then_0
            (Timeline|ChargeUpGun Reverse))
          (:then_1
            (CallFunction|DecreaseHeat)))))))

(event EventSetReload
  ;[1 1 1] Disable Reload when overheated
  (if (not (Variables|Default|GetIsOverheated))
    (|CallParentFunction)))

(event EventBeginPlay
  (|CallParentFunction)
  (Variables|Default|SetWeaponStruct (Variables|Default|GetWeaponStruct)))

(event EventFireBullet
  ;[1 1 1] Overheat when shooting
  (if (not (Variables|Default|GetIsOverheated))
    (|CallParentFunction)
    (if (not (Variables|Default|GetIsReloading))
      (bind _output_get (Variables|Default|SetCurrentHeat (+ (Variables|Default|GetCurrentHeat) (* (Variables|Default|GetFireRate) 0.4))))
      (Variables|Default|SetIsOverheated (>= (Math|Float|Clamp(Float) _output_get) 1.0)))))

(fn ConstructionScript
  (|CallParentFunction))
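; Master weapon actor that fires bullets for its parent BP_ThirdPersonCharacter.
; FireWeapon and StopFire only toggle IsFiring; nothing in these graphs calls FireBullet.
; FireBullet triggers the character's shot effects, then line-traces from the player camera with random spread from WeaponStruct, drawing debug lines.
; Only on a blocking hit, it spawns an impact emitter and a BP_Bullet at the barrel, aimed at the hit point.
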(event Custom|Fire%20Weapon
  (Variables|Default|SetIsFiring true))

(event Custom|StopFire
  (Variables|Default|SetIsFiring false))

(event EventBeginPlay
  (Utilities|Struct|SetmembersinS_WeaponStructs (Variables|Default|GetWeaponStruct)))

(fn ConstructionScript)

(fn FireBullet
  (bind _weaponstruct (Variables|Default|GetWeaponStruct))
  (bind _barrelreference (Variables|Default|GetBarrelReference))
  (bind _bulletspread (Utilities|Struct|BreakS_WeaponStructs _weaponstruct))
  (bind _returnvalue (Transformation|GetWorldLocation _barrelreference))
  (bind _returnvalue_2 (* _bulletspread -1.0))
  ;[1 1 1] Shoot Projectile
  (bind _asbp_third_person_character (Utilities|Casting|CastToBP_ThirdPersonCharacter (Actor|GetParentActor)))
  (Default|ShootParticle+Sound _asbp_third_person_character)
  (bind (_outhit _returnvalue_3) (Collision|LineTraceForObjects (Transformation|GetWorldLocation (Variables|/Game/Spawn_System/Blueprints/Character/BP_ThirdPersonCharacter.BP_ThirdPersonCharacter_C|GetPlayerCamera _asbp_third_person_character)) (+ (+ (Transformation|GetWorldLocation (Variables|/Game/Spawn_System/Blueprints/Character/BP_ThirdPersonCharacter.BP_ThirdPersonCharacter_C|GetPlayerCamera _asbp_third_person_character)) (* (Math|Vector|GetForwardVector (Variables|/Game/Spawn_System/Blueprints/Character/BP_ThirdPersonCharacter.BP_ThirdPersonCharacter_C|GetPlayerCamera _asbp_third_person_character)) 1e+04)) (Math|Vector|MakeVector (Math|Random|RandomFloatinRange _returnvalue_2 _bulletspread) (Math|Random|RandomFloatinRange _returnvalue_2 _bulletspread) (Math|Random|RandomFloatinRange _returnvalue_2 _bulletspread))) (Utilities|Array|MakeArray "ObjectTypeQuery3" "ObjectTypeQuery1") true 0 "ForDuration"))
  (if (.bBlockingHit (Collision|BreakHitResult _outhit))
    (Effects|SpawnEmitteratLocation "/Game/Spawn_System/Particles/P_Shoot_Effect.P_Shoot_Effect" (.ImpactPoint (Collision|BreakHitResult _outhit)))
    (Game|SpawnActorfromClass "/Game/Blueprints/Weapons/Projectiles/BP_Bullet.BP_Bullet_C" (Math|Transform|MakeTransform _returnvalue (Math|Rotator|FindLookatRotation _returnvalue (Math|Vector|SelectVector (.ImpactPoint (Collision|BreakHitResult _outhit)) (.TraceEnd (Collision|BreakHitResult _outhit)) _returnvalue_3))) "AlwaysSpawn" 0 0)))